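; BP_Door is an interactable door in the stealth game that toggles open or closed when the custom third-person character enters its box collision.
; If Unlocked, each entry flips IsOpen and plays or reverses the DoorOpen timeline, which drives the door mesh's relative yaw.
; Otherwise it prints a locked message.
; A Player flag tracks whether the character is inside the box.
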(event OnComponentBeginOverlap(Boxcollision)
  (params (OverlappedComponent :type Primitive%20Component%20Object%20Reference) (OtherActor :type Actor%20Object%20Reference) (OtherComp :type Primitive%20Component%20Object%20Reference) (OtherBodyIndex :type Integer) (bFromSweep :type Boolean) (SweepResult :type Hit%20Result%20Structure%20%28by%20ref%29))
  (Utilities|Casting|CastToBP_ThirdPersonCharacterCustom OtherActor)
  (Variables|Default|SetPlayer? true)
  (if (Variables|Default|GetUnlocked)
    (if (Variables|Default|GetIsOpen)
      (Variables|Default|SetIsOpen false)
      (bind _doormovement (Timeline|DoorOpen Reverse)
        (:Update
          (Transformation|SetRelativeRotation (Variables|Default|GetSM_Door) (Math|Rotator|MakeRotator 0.0 0.0 _doormovement) false false)))
      (else
        (Variables|Default|SetIsOpen true)
        (Timeline|DoorOpen Play)))
    (else
      (Development|PrintString "Door Locked"))))

(event OnComponentEndOverlap(Boxcollision)
  (params (OverlappedComponent :type Primitive%20Component%20Object%20Reference) (OtherActor :type Actor%20Object%20Reference) (OtherComp :type Primitive%20Component%20Object%20Reference) (OtherBodyIndex :type Integer))
  (Utilities|Casting|CastToBP_ThirdPersonCharacterCustom OtherActor)
  (Variables|Default|SetPlayer? false))

(event Collision|EventActorBeginOverlap
  (params (OtherActor :type Actor%20Object%20Reference)))

(event EventTick
  (params (DeltaSeconds :type Float%20%28single-precision%29)))

(fn ConstructionScript)