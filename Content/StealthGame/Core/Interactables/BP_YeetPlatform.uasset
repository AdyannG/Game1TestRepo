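; BP_YeetPlatform is a moving platform that shuttles back and forth between its Start and End component positions from BeginPlay.
; A Timeline lerps the platform's relative location without sweep, and a FlipFlop on Finished alternates reverse and forward playback after a pause.
; Delays chained off the Timeline Update briefly flash the platform emissive green at intervals during travel, then restore its table material.
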(event EventBeginPlay
  (bind _floattrack (Timeline|Timeline PlayFromStart)
    (:Update
      (Transformation|SetRelativeLocation (Variables|Default|GetPlatform) (Math|Vector|Lerp(Vector) (Variables|/Script/Engine.SceneComponent|GetRelativeLocation (Variables|Default|GetStart)) (Variables|/Script/Engine.SceneComponent|GetRelativeLocation (Variables|Default|GetEnd)) _floattrack) false false)
      (Utilities|FlowControl|Delay 0.6)
      (Rendering|Material|SetMaterial (Variables|Default|GetPlatform) 0 "/Game/StealthGame/MaterialLibrary/Coding1Materials/MI_EmmissveGreen.MI_EmmissveGreen")
      (Utilities|FlowControl|Delay 0.1)
      (Rendering|Material|SetMaterial (Variables|Default|GetPlatform) 0 "/Game/StealthGame/Core/StarterContent/Props/Materials/M_TableRound.M_TableRound"))
    (:Finished
      (Utilities|FlowControl|Delay 2.0)
      (Utilities|FlowControl|FlipFlop ; If A, Reverse from End\nif B, Start from Beginning
        (:A
          (Timeline|Timeline ReverseFromEnd))
        (:B
          (Timeline|Timeline PlayFromStart))))))

(fn ConstructionScript)