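; BP_PowerCell is a pickup item in the stealth game that the third-person character can carry and drop.
; Overlapping its trigger asks the character to pick it up, and Pickup attaches the cell mesh to the hand_r socket with collision off.
; Drop detaches the cell, re-enables collision and physics, and restores its world location so it falls in place.
; PrimaryAction is empty, leaving a placeholder health-and-destroy chain unconnected.
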(event OnComponentBeginOverlap(PickupTrigger)
  (params (OverlappedComponent :type Primitive%20Component%20Object%20Reference) (OtherActor :type Actor%20Object%20Reference) (OtherComp :type Primitive%20Component%20Object%20Reference) (OtherBodyIndex :type Integer) (bFromSweep :type Boolean) (SweepResult :type Hit%20Result%20Structure%20%28by%20ref%29))
  (bind _asbp_third_person_character_custom (Utilities|Casting|CastToBP_ThirdPersonCharacterCustom OtherActor))
  (Default|TrytoPickUp _asbp_third_person_character_custom self))

(event EventPickup
  (params (ParentMesh :type Skeletal%20Mesh%20Component%20Object%20Reference))
  (Transformation|AttachComponentToComponent (Variables|Default|GetCell) ParentMesh "hand_r" "SnapToTarget" "KeepRelative" "KeepRelative" true)
  (Collision|SetCollisionEnabled (Variables|Default|GetCell) "NoCollision") ; Collide with the ground please
)

(event EventDrop
  (bind _cell (Variables|Default|GetCell))
  (Variables|Default|SetDrop%20Location (Transformation|GetWorldLocation _cell))
  (Transformation|DetachFromComponent _cell "KeepRelative" "KeepRelative" "KeepRelative" true) ; Don't follow the hand anymore
  (Physics|SetSimulatePhysics (Variables|Default|GetCell) true) ; use gravity to fall
  (Collision|SetCollisionEnabled (Variables|Default|GetCell) "QueryAndPhysics") ; Collide with the ground please
  (Transformation|SetWorldLocation (Variables|Default|GetCell) (Variables|Default|GetDrop%20Location) false false) ; To prevent the can from going to world origin
)

(event EventPrimaryAction
  (params (ref_thirdPersonCharCustom :type BP%20Third%20Person%20Character%20Custom%20Object%20Reference))
  ;[1 1 1] Comment
)

(fn ConstructionScript)